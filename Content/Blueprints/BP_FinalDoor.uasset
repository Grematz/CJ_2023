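; BP_FinalDoor is the level's final exit door, which wins the game when opened with the magnetic key after activation.
; Activate sets the activated flag and turns the spotlight green.
; Interact checks the character's key and activation, then either pauses and shows the win screen or plays a denied sound.
; A TryOpen flag blocks repeat interactions and resets only after a denial, so interacting without the key leaves it set.
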(event `Activate`
  (set `self.Activated` true)
  (`LightComponent.SetLightColor` (`self.SpotLight`) (struct :`G` 1.0 :`B` 0.133136 :`A` 1.0) true))

(event `/Game/Blueprints/BPI_Interact.Interact`
  (params (Chara :type "/Game/FirstPerson/Blueprints/BP_FirstPersonCharacter Object Reference"))
  (if (not (`self.TryOpen`))
    (set `self.TryOpen` true)
    (if (`/Game/FirstPerson/Blueprints/BP_FirstPersonCharacter.KeyMagneticIsTake` Chara)
      (if (`self.Activated`)
        (`GameplayStatics.PlaySound2D` "/Game/Audio/Elecronic/KeyCardOpen_Cue.KeyCardOpen_Cue" 1.0 1.0 0.0 null null)
        (`KismetSystemLibrary.Delay` 1.0)
        (`GameplayStatics.SetGamePaused` true)
        (bind _returnvalue (`|CreateWidget` "/Game/Blueprints/Widgets/UW_WinScreen.UW_WinScreen_C"))
        (`UserWidget.AddToViewport` _returnvalue 0)
        (set `PlayerController.bShowMouseCursor` true (`GameplayStatics.GetPlayerController` 0))
        (else
          (`GameplayStatics.PlaySound2D` "/Game/Audio/Elecronic/KeyCardDenied_Cue.KeyCardDenied_Cue" 1.0 1.0 0.0 null null)
          (`KismetSystemLibrary.Delay` 1.0)
          (set `self.TryOpen` false))))))

(fn `UserConstructionScript`)