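; Light bulb collectible that the player can pick up.
; On BeginPlay it runs the parent logic and sets its object name to "Light Bulb".
; Each Tick it polls whether it is pickable and the referenced character is picking an item, then plays the battery pickup sound at its location and destroys itself.
; It adds no inventory or counter update of its own.
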(event `self.ReceiveBeginPlay`
  (`parent.ReceiveBeginPlay`)
  (set `self.ObjectName` "Light Bulb"))

(event `self.ReceiveTick`
  (params (DeltaSeconds :type "Float (single-precision)"))
  (if (`self.IsPickable`)
    (if (`/Game/FirstPerson/Blueprints/BP_FirstPersonCharacter.PickingItem` (`self.CharacterRef`))
      (`GameplayStatics.PlaySoundAtLocation` "/Game/Audio/Environment/PickUpBattery_Cue.PickUpBattery_Cue" (`self.K2_GetActorLocation`) (struct) 1.0 1.0 0.0 null null null null)
      (`self.K2_DestroyActor`))))

(fn `UserConstructionScript`
  (`parent.UserConstructionScript`))