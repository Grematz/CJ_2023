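; BP_Collectible_Key is a key pickup that records itself on the player character when collected.
; It sets its object name to "Key" and each Tick checks whether it is pickable while the character is picking an item.
; A DoOnce then plays the pickup sound, flags its KeyNumber slot in the character's Keys array and destroys the actor.
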(event `self.ReceiveBeginPlay`
  (`parent.ReceiveBeginPlay`)
  (set `self.ObjectName` "Key"))

(event `self.ReceiveTick`
  (params (DeltaSeconds :type "Float (single-precision)"))
  (if (`self.IsPickable`)
    (if (`/Game/FirstPerson/Blueprints/BP_FirstPersonCharacter.PickingItem` (`self.CharacterRef`))
      (`/Engine/EditorBlueprintResources/StandardMacros.DoOnce` false
        (:`Completed`
          (`GameplayStatics.PlaySoundAtLocation` "/Game/Audio/Environment/TakeKey_Cue.TakeKey_Cue" (`self.K2_GetActorLocation`) (struct) 1.0 1.0 0.0 null null null null)
          (`KismetArrayLibrary.Array_Set` (`/Game/FirstPerson/Blueprints/BP_FirstPersonCharacter.Keys` (`self.CharacterRef`)) (`self.KeyNumber`) true)
          (`self.K2_DestroyActor`))))))

(fn `UserConstructionScript`
  (`parent.UserConstructionScript`))