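; Interactable door that swings open once, optionally gated by a key and by electrical power.
; Interact checks the NeedKey and NeedElec flags, reading power from the first BP_Boitier found and the key from the character's KeyIsTake.
; Success plays sounds and a Timeline yaws Scene1 from the mesh's starting rotation; failure plays a locked sound and re-enables attempts after a delay.
; An older per-door-number key check remains unconnected.
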(event `self.ReceiveBeginPlay`
  (set `self.OriginValue` (`SceneComponent.K2_GetComponentRotation` (`self.StaticMesh`))))

(event `/Game/Blueprints/BPI_Interact.Interact`
  (params (Chara :type "/Game/FirstPerson/Blueprints/BP_FirstPersonCharacter Object Reference"))
  (bind (_originvalue_roll _originvalue_pitch _originvalue_yaw) (`KismetMathLibrary.BreakRotator` (`self.OriginValue`)))
  (if (not (`self.TryOpen`))
    (set `self.TryOpen` true)
    (if (`self.Opened`)
      _
      (elif (`self.NeedKey`)
        (if (`self.NeedElec`)
          (bind _returnvalue (`GameplayStatics.GetActorOfClass` "/Game/Blueprints/BP_Boitier.BP_Boitier_C"))
          (if (`/Game/Blueprints/BP_Boitier.On` _returnvalue)
            (if (`/Game/FirstPerson/Blueprints/BP_FirstPersonCharacter.KeyIsTake` Chara) :!label _label
              (`GameplayStatics.PlaySoundAtLocation` "/Game/Sounds/UnlockDoor.UnlockDoor" (0.0 0.0 0.0) (struct) 1.0 1.0 0.0 null null null null)
              (`KismetSystemLibrary.Delay` 1.0)
              (`GameplayStatics.PlaySoundAtLocation` "/Game/Sounds/grincement-de-porte-suspense-bruitage-gratuit_Cue.grincement-de-porte-suspense-bruitage-gratuit_Cue" (`SceneComponent.K2_GetComponentLocation` (`self.StaticMesh`)) (struct) 1.0 1.0 0.0 null null null null :!label _label_2)
              (set `self.Opened` true)
              (bind (_direction _newtrack_0) (`Timeline|Timeline`)
                (:`Update`
                  (`SceneComponent.K2_SetWorldRotation` (`self.Scene1`) (`KismetMathLibrary.MakeRotator` 0.0 0.0 (+ _originvalue_yaw _newtrack_0)) false false)))
              (else
                (`GameplayStatics.PlaySound2D` "/Game/Sounds/doorlocked.doorlocked" 1.0 1.0 0.0 null null :!label _label_3)
                (`KismetSystemLibrary.Delay` 1.0)
                (set `self.TryOpen` false)))
            (else
              (goto _label_3)))
          (else
            (goto _label)))
        (else
          (goto _label_2))))))

(fn `UserConstructionScript`)