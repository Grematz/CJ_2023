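; BP_Ampoule is a light bulb that freezes mannequin enemies by deactivating their AI while lit.
; TurnOn, optionally run at BeginPlay, either shows the point light steadily or, with Click set, starts a looping timer that flickers it randomly.
; Each flicker deactivates or reactivates only the first mannequin in the sphere to match the light.
; Actors entering the sphere while it is lit have their mannequin AI deactivated, with no handling on exit.
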(event `self.ReceiveBeginPlay`
  (if (`self.OnBegin`)
    (`self.TurnOn`)))

(event `TurnOn`
  (if (`self.Click`)
    (`KismetSystemLibrary.K2_SetTimerDelegate` (delegate `CustomEvent`) 0.1 true)
    (set `self.TurnedOn` true)
    (else
      (`SceneComponent.SetVisibility` (`self.PointLight`) true false)
      (set `self.TurnedOn` true))))

(event `CustomEvent`
  (bind _pointlight (`self.PointLight`))
  (bind _returnvalue (`SceneComponent.IsVisible` _pointlight))
  (bind _returnvalue_2 (`AIBlueprintHelperLibrary.GetAIController` (`|GetArrayItem` (`PrimitiveComponent.GetOverlappingActors` (`self.Sphere`) "/Game/Blueprints/Mannequin/BP_Mannequin.BP_Mannequin_C"))))
  (if (`KismetMathLibrary.RandomBoolWithWeight` 0.3)
    (`SceneComponent.SetVisibility` _pointlight (not _returnvalue) false)
    (if _returnvalue
      (bind _asaic_mannequin (cast `/Game/Blueprints/Mannequin/AIC_Mannequin` _returnvalue_2))
      (`/Game/Blueprints/Mannequin/AIC_Mannequin.Deactivate` _asaic_mannequin)
      (else
        (bind _asaic_mannequin_2 (cast `/Game/Blueprints/Mannequin/AIC_Mannequin` _returnvalue_2))
        (`/Game/Blueprints/Mannequin/AIC_Mannequin.Activate` _asaic_mannequin_2)))))

(event `self.Sphere.OnComponentBeginOverlap`
  (params (OverlappedComponent :type "PrimitiveComponent Object Reference") (OtherActor :type "Actor Object Reference") (OtherComp :type "PrimitiveComponent Object Reference") (OtherBodyIndex :type Integer) (bFromSweep :type Boolean) (SweepResult :type "HitResult Structure (by ref)"))
  (if (`SceneComponent.IsVisible` (`self.PointLight`))
    (bind _asaic_mannequin (cast `/Game/Blueprints/Mannequin/AIC_Mannequin` (`AIBlueprintHelperLibrary.GetAIController` OtherActor)))
    (`/Game/Blueprints/Mannequin/AIC_Mannequin.Deactivate` _asaic_mannequin)))

(fn `UserConstructionScript`)